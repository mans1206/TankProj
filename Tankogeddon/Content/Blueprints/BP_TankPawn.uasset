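; Player tank pawn Blueprint whose graph handles UI: a game-over widget on destruction and hotkey-driven menus.
; M flip-flops the main menu through MyHUD, pausing on open with no unpause here.
; N and C flip-flop tank and spawned lists, but create a new widget each press, so removal targets that new instance.
; All three created widgets share the WGameOver variable.
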(event `self.ReceiveBeginPlay`)

(event `self.ReceiveTick`
  (params (DeltaSeconds :type "Float (single-precision)")))

(event `self.ReceiveDestroyed`
  (bind _astank_player_controller (cast `TankPlayerController` (`GameplayStatics.GetPlayerController` 0)))
  (bind _returnvalue (`|CreateWidget` "/Game/Widgets/W_GameOVer.W_GameOver_C" _astank_player_controller))
  (set `self.W_GameOver` _returnvalue)
  (`UserWidget.AddToViewport` _returnvalue 0))

(event `Key|M`
  (params (Key :type "Key Structure"))
  (:`Pressed`
    (bind _asmy_hud (cast `MyHUD` (`PlayerController.GetHUD` (`GameplayStatics.GetPlayerController` 0))))
    (`/Engine/EditorBlueprintResources/StandardMacros.FlipFlop`
      (:`A`
        (`MyHUD.AddWidgetToViewportByClass` _asmy_hud "/Game/Widgets/W_MainMenuC++.W_MainMenuC++_C" 0)
        (`GameplayStatics.SetGamePaused` true))
      (:`B`
        (`MyHUD.RemoveCurrentWidgetFromViewport` _asmy_hud)))))

(event `Key|N`
  (params (Key :type "Key Structure"))
  (:`Pressed`
    (bind _astank_player_controller (cast `TankPlayerController` (`GameplayStatics.GetPlayerController` 0)))
    (bind _returnvalue (`|CreateWidget` "/Game/Widgets/WBP_TankList.WBP_TankList_C" _astank_player_controller))
    (set `self.W_GameOver` _returnvalue)
    (`/Engine/EditorBlueprintResources/StandardMacros.FlipFlop`
      (:`A`
        (`UserWidget.AddToViewport` _returnvalue 0))
      (:`B`
        (`Widget.RemoveFromParent` _returnvalue)))))

(event `Key|C`
  (params (Key :type "Key Structure"))
  (:`Pressed`
    (bind _astank_player_controller (cast `TankPlayerController` (`GameplayStatics.GetPlayerController` 0)))
    (bind _returnvalue (`|CreateWidget` "/Game/Widgets/WBP_SpawnedList.WBP_SpawnedList_C" _astank_player_controller))
    (set `self.W_GameOver` _returnvalue)
    (`/Engine/EditorBlueprintResources/StandardMacros.FlipFlop`
      (:`A`
        (`UserWidget.AddToViewport` _returnvalue 0))
      (:`B`
        (`Widget.RemoveFromParent` _returnvalue)))))

(fn `Remove from parent`)

(fn `UserConstructionScript`)